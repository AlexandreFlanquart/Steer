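; BP_Pawn is a player-controlled pawn that moves freely along the world X and Y axes and can trigger a mode switch.
; Forward and Right axis inputs offset the actor location each event by the axis value times Spd, without sweep or delta-time scaling.
; Pressing SwitchMode finds all BP_PawnPath actors and calls ChangeMode on the first one, with no check that one exists.
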(event `InputAxis|Forward`
  (params (AxisValue :type "Float (single-precision)"))
  (`self.K2_SetActorLocation` (+ (`self.K2_GetActorLocation`) (`KismetMathLibrary.MakeVector` (* AxisValue (`self.spd`))))))

(event `InputAxis|Right`
  (params (AxisValue :type "Float (single-precision)"))
  (`self.K2_SetActorLocation` (+ (`self.K2_GetActorLocation`) (`KismetMathLibrary.MakeVector` 0.0 (* AxisValue (`self.spd`))))))

(event `InputAction|SwitchMode`
  (params (Key :type "Key Structure"))
  (:`Pressed`
    (bind _outactors (`GameplayStatics.GetAllActorsOfClass` "/Game/Blueprint/BP_PawnPath.BP_PawnPath_C"))
    (`MyPawnPath.ChangeMode` (`|GetArrayItem` _outactors))))

(fn `UserConstructionScript`)